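; Ammo pickup collectable that refills a shooter character's reserve ammo on contact.
; Its Box overlap accepts only BP_ShooterCharacter and adds a fixed amount to that character's AmmoBank.
; It then starts a reload on the current weapon if it is empty and not already reloading, and destroys itself.
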(event OnComponentBeginOverlap(Box)
  (params (OverlappedComponent :type Primitive%20Component%20Object%20Reference) (OtherActor :type Actor%20Object%20Reference) (OtherComp :type Primitive%20Component%20Object%20Reference) (OtherBodyIndex :type Integer) (bFromSweep :type Boolean) (SweepResult :type Hit%20Result%20Structure%20%28by%20ref%29))
  (bind _asbp_shooter_character (Utilities|Casting|CastToBP_ShooterCharacter OtherActor))
  (Utilities|FlowControl|Sequence
    (:then_0
      (Variables|/Game/Variant_Shooter/Blueprints/BP_ShooterCharacter.BP_ShooterCharacter_C|SetAmmo%20Bank _asbp_shooter_character (+ (Variables|/Game/Variant_Shooter/Blueprints/BP_ShooterCharacter.BP_ShooterCharacter_C|GetAmmo%20Bank _asbp_shooter_character) 12)))
    (:then_1
      (if (not (Variables|/Game/Variant_Shooter/Blueprints/Pickups/BP_ShooterWeaponBase.BP_ShooterWeaponBase_C|GetReloading (Variables|/Game/Variant_Shooter/Blueprints/BP_ShooterCharacter.BP_ShooterCharacter_C|GetCurrent%20Weapon _asbp_shooter_character)))
        (if (== (Variables|/Game/Variant_Shooter/Blueprints/Pickups/BP_ShooterWeaponBase.BP_ShooterWeaponBase_C|GetCurrent%20Bullets (Variables|/Game/Variant_Shooter/Blueprints/BP_ShooterCharacter.BP_ShooterCharacter_C|GetCurrent%20Weapon _asbp_shooter_character)) 0)
          (Default|StartReloading (Variables|/Game/Variant_Shooter/Blueprints/BP_ShooterCharacter.BP_ShooterCharacter_C|GetCurrent%20Weapon _asbp_shooter_character)))))
    (:then_2
      (Actor|DestroyActor))))

(event EventBeginPlay)

(event Collision|EventActorBeginOverlap
  (params (OtherActor :type Actor%20Object%20Reference)))

(event EventTick
  (params (DeltaSeconds :type Float%20%28single-precision%29)))

(fn ConstructionScript)