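; BP_CabbageCoin is a collectable coin that awards a cabbage coin to the shooter character who picks it up.
; On BeginPlay a Timeline moves the Cylinder along a Spline in local space, restarting from zero whenever it finishes to loop the motion.
; When the Box overlaps a BP_ShooterCharacter, it calls AddCabbageCoin on that character and destroys the coin.
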(event OnComponentBeginOverlap(Box)
  (params (OverlappedComponent :type Primitive%20Component%20Object%20Reference) (OtherActor :type Actor%20Object%20Reference) (OtherComp :type Primitive%20Component%20Object%20Reference) (OtherBodyIndex :type Integer) (bFromSweep :type Boolean) (SweepResult :type Hit%20Result%20Structure%20%28by%20ref%29))
  (bind _asbp_shooter_character (Utilities|Casting|CastToBP_ShooterCharacter OtherActor))
  (Default|AddCabbageCoin _asbp_shooter_character)
  (Actor|DestroyActor))

(event EventBeginPlay
  (bind _новая_дорожка_0 (Timeline|Timeline Play)
    (:Update
      (Transformation|SetRelativeLocation (Variables|Default|GetCylinder) (Spline|GetLocationatTime (Variables|Default|GetSpline) _новая_дорожка_0 "Local" false) false false))
    (:Finished
      (Components|Timeline|SetNewTime (Variables|Default|GetTimeline) 0.0)
      (Timeline|Timeline Play))))

(event EventTick
  (params (DeltaSeconds :type Float%20%28single-precision%29)))

(fn ConstructionScript)