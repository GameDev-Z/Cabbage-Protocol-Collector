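; Enemy character that patrols, chases and shoots BP_ShooterCharacter, scripted entirely in the event graph.
; It walks between random navigable points until ChaseRange sees the player and starts pursuit, while ShootRange triggers turning and rate-limited projectile fire.
; DoOnce gates and delays switch animations and walk speed before falling back to patrol.
; Each hit costs one health; death spawns a coin and possibly ammo, then ragdolls before destruction.
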(event OnSeePawn(ChaseRange)
  (params (Pawn :type Pawn%20Object%20Reference))
  ;[0.15 0.15 0.15 0.5] Chase
  (bind _asbp_shooter_character (Utilities|Casting|CastToBP_ShooterCharacter Pawn))
  (if (not (Variables|Default|GetIsShooting))
    (Utilities|FlowControl|Sequence
      (:then_0
        (Utilities|FlowControl|DoOnce false
          (:Completed
            (Components|Animation|PlayAnimation (Variables|Character|GetMesh) "/Game/Characters/Mannequins/Anims/Unarmed/Jog/MF_Unarmed_Jog_Fwd.MF_Unarmed_Jog_Fwd" true)
            (Variables|/Script/Engine.CharacterMovementComponent|SetMaxWalkSpeed (Variables|Character|GetCharacterMovement) 3e+02))))
      (:then_1
        (AI|AIMoveTo self "0, 0, 0" _asbp_shooter_character 5.0 false
          (:then
            (Utilities|FlowControl|RetriggerableDelay 3.0)
            (Components|Animation|PlayAnimation (Variables|Character|GetMesh) "/Game/Characters/Mannequins/Anims/Unarmed/Walk/MF_Unarmed_Walk_Fwd.MF_Unarmed_Walk_Fwd" true)
            (Variables|/Script/Engine.CharacterMovementComponent|SetMaxWalkSpeed (Variables|Character|GetCharacterMovement) 2e+02)
            (CallFunction|CanChaseAgain)
            (CallFunction|Patrol)))))))

(event OnSeePawn(ShootRange)
  (params (Pawn :type Pawn%20Object%20Reference))
  ;[0.15 0.15 0.15 0.5] Attack
  (bind _asbp_shooter_character (Utilities|Casting|CastToBP_ShooterCharacter Pawn))
  (Utilities|FlowControl|Sequence
    (:then_0
      (Utilities|FlowControl|DoOnce false
        (:Completed
          (Components|Animation|PlayAnimation (Variables|Character|GetMesh) "/Game/Characters/Mannequins/Anims/Pistol/MF_Pistol_Idle_ADS.MF_Pistol_Idle_ADS" true)
          (Variables|/Script/Engine.CharacterMovementComponent|SetMaxWalkSpeed (Variables|Character|GetCharacterMovement) 0.0)
          (Variables|Default|SetIsShooting true))))
    (:then_1
      (Transformation|SetActorRotation (Math|Rotator|FindLookatRotation (Transformation|GetActorLocation) (Transformation|GetActorLocation _asbp_shooter_character)))
      (Utilities|FlowControl|Delay 0.2)
      (if (> (- (Utilities|Time|GetGameTimeinSeconds) (Variables|Default|GetTime%20of%20Last%20Shot)) (Variables|Default|GetRefire%20Rate))
        (Game|SpawnActorfromClass "/Game/Variant_Shooter/Blueprints/Pickups/Projectiles/BP_ShooterProjectile_Bullet.BP_ShooterProjectile_Bullet_C" (Transformation|GetWorldTransform (Variables|Default|GetCool%20arrow)) "Undefined" "MultiplyWithRoot" 0 0)
        (Variables|Default|SetTime%20of%20Last%20Shot (Utilities|Time|GetGameTimeinSeconds)))
      (Components|Animation|PlayAnimation (Variables|Character|GetMesh) "/Game/Characters/Mannequins/Anims/Unarmed/Walk/MF_Unarmed_Walk_Fwd.MF_Unarmed_Walk_Fwd" true)
      (Variables|/Script/Engine.CharacterMovementComponent|SetMaxWalkSpeed (Variables|Character|GetCharacterMovement) 2e+02)
      (CallFunction|CanShootAgain)
      (Variables|Default|SetIsShooting false)
      (CallFunction|Patrol))))

(event Custom|Patrol
  ;[0.15 0.15 0.15 0.5] Patrol
  (if (not (Variables|Default|GetIsShooting))
    (Components|Animation|PlayAnimation (Variables|Character|GetMesh) "/Game/Characters/Mannequins/Anims/Unarmed/Walk/MF_Unarmed_Walk_Fwd.MF_Unarmed_Walk_Fwd" true)
    (bind _randomlocation (Class|NavigationSystemV1|GetRandomLocationinNavigableRadius (Transformation|GetActorLocation) 5e+02 0 0))
    (AI|AIMoveTo self _randomlocation 0 5.0 false
      (:OnSuccess
        (Components|Animation|PlayAnimation (Variables|Character|GetMesh) "/Game/Characters/Mannequins/Anims/Unarmed/BS_Idle_Walk_Run.BS_Idle_Walk_Run" true)
        (Utilities|FlowControl|Delay 3.0)
        (CallFunction|Patrol)))))

(event Custom|Die
  (bind _returnvalue (Transformation|GetActorTransform))
  (bind _mesh (Variables|Character|GetMesh))
  (bind _charactermovement (Variables|Character|GetCharacterMovement))
  (Utilities|FlowControl|DoOnce false
    (:Completed
      (Game|SpawnActorfromClass "/Game/Collectables/BP_CabbageCoin.BP_CabbageCoin_C" _returnvalue "Undefined" "MultiplyWithRoot" 0 0)
      (if (Math|Random|RandomBool)
        (Game|SpawnActorfromClass "/Game/Collectables/BP_AmmoBox.BP_AmmoBox_C" _returnvalue "Undefined" "MultiplyWithRoot" 0 0))
      (Collision|SetCollisionEnabled (Variables|Collision|GetCapsuleComponent) "NoCollision")
      (Components|Movement|StopMovementImmediately _charactermovement)
      (Class|NavMovementInterface|StopActiveMovement _charactermovement)
      (Collision|SetCollisionProfileName _mesh "Ragdoll" true :!class /Script/Engine.PrimitiveComponent)
      (Physics|SetSimulatePhysics _mesh true)
      (Class|SkeletalMeshComponent|SetPhysicsBlendWeight _mesh 1.0)
      (Components|DestroyComponent (Variables|Default|GetShootRange))
      (Utilities|FlowControl|Delay 1e+01)
      (Actor|DestroyActor))))

(event Custom|Can%20chase%20again
  ;[0.15 0.15 0.15 0.5] Chase
  (Utilities|FlowControl|DoOnce false) ; enters at Reset
)

(event Custom|Can%20Shoot%20again
  ;[0.15 0.15 0.15 0.5] Attack
  (Utilities|FlowControl|DoOnce false) ; enters at Reset
)

(event EventBeginPlay
  (CallFunction|Patrol)
  (Variables|/Script/Engine.CharacterMovementComponent|SetMaxWalkSpeed (Variables|Character|GetCharacterMovement) 2e+02)
  (Variables|Default|SetHealth 3)
  (Variables|Default|SetCanShoot true)
  (Variables|Default|SetRefire%20Rate 1.0))

(event Game|Damage|EventAnyDamage
  (params (Damage :type Float%20%28single-precision%29) (DamageType :type Damage%20Type%20Object%20Reference) (InstigatedBy :type Controller%20Object%20Reference) (DamageCauser :type Actor%20Object%20Reference))
  ;[0.15 0.15 0.15 0.5] Taking damage
  (bind _output_get (Variables|Default|SetHealth (- (Variables|Default|GetHealth) 1)))
  (if (== _output_get 0)
    (CallFunction|Die)))

(fn ConstructionScript)