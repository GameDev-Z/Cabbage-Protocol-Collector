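; Map generator prop actor that randomly thins out its own set of two box and two pillar components for variation.
; On BeginPlay, each component gets an independent weighted random roll and is destroyed about one time in three.
; The variation is decided at runtime, as the construction script is empty.
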(event EventBeginPlay
  (Utilities|FlowControl|Sequence
    (:then_0
      (if (Math|Random|RandomBoolwithWeight 0.333333)
        (Components|DestroyComponent (Variables|Default|GetBox))))
    (:then_1
      (if (Math|Random|RandomBoolwithWeight 0.333333)
        (Components|DestroyComponent (Variables|Default|GetBox1))))
    (:then_2
      (if (Math|Random|RandomBoolwithWeight 0.333333)
        (Components|DestroyComponent (Variables|Default|GetPillar))))
    (:then_3
      (if (Math|Random|RandomBoolwithWeight 0.333333)
        (Components|DestroyComponent (Variables|Default|GetPillar1))))))

(fn ConstructionScript)