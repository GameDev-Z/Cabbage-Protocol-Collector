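; BP_ExitGeneratorEasy is a level exit in the map generator that moves the player on to the next level.
; Two overlap triggers, HardLvl and EasyLvl, react only to BP_ShooterCharacter and increment its PassLvl counter.
; Both run identical logic: open BossLvl when PassLvl equals MaxLvl, otherwise EasyLvl, so the HardLvl trigger also leads to EasyLvl.
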(event OnComponentBeginOverlap(HardLvl)
  (params (OverlappedComponent :type Primitive%20Component%20Object%20Reference) (OtherActor :type Actor%20Object%20Reference) (OtherComp :type Primitive%20Component%20Object%20Reference) (OtherBodyIndex :type Integer) (bFromSweep :type Boolean) (SweepResult :type Hit%20Result%20Structure%20%28by%20ref%29))
  (bind _asbp_shooter_character (Utilities|Casting|CastToBP_ShooterCharacter OtherActor))
  (Variables|/Game/Variant_Shooter/Blueprints/BP_ShooterCharacter.BP_ShooterCharacter_C|SetPassLvl _asbp_shooter_character (+ (Variables|/Game/Variant_Shooter/Blueprints/BP_ShooterCharacter.BP_ShooterCharacter_C|GetPassLvl _asbp_shooter_character) 1))
  (if (== (Variables|/Game/Variant_Shooter/Blueprints/BP_ShooterCharacter.BP_ShooterCharacter_C|GetPassLvl _asbp_shooter_character) (Variables|/Game/Variant_Shooter/Blueprints/BP_ShooterCharacter.BP_ShooterCharacter_C|GetMaxLvl _asbp_shooter_character))
    (Game|OpenLevel(byName) "BossLvl")
    (else
      (Game|OpenLevel(byName) "EasyLvl"))))

(event OnComponentBeginOverlap(EasyLvl)
  (params (OverlappedComponent :type Primitive%20Component%20Object%20Reference) (OtherActor :type Actor%20Object%20Reference) (OtherComp :type Primitive%20Component%20Object%20Reference) (OtherBodyIndex :type Integer) (bFromSweep :type Boolean) (SweepResult :type Hit%20Result%20Structure%20%28by%20ref%29))
  (bind _asbp_shooter_character (Utilities|Casting|CastToBP_ShooterCharacter OtherActor))
  (Variables|/Game/Variant_Shooter/Blueprints/BP_ShooterCharacter.BP_ShooterCharacter_C|SetPassLvl _asbp_shooter_character (+ (Variables|/Game/Variant_Shooter/Blueprints/BP_ShooterCharacter.BP_ShooterCharacter_C|GetPassLvl _asbp_shooter_character) 1))
  (if (== (Variables|/Game/Variant_Shooter/Blueprints/BP_ShooterCharacter.BP_ShooterCharacter_C|GetPassLvl _asbp_shooter_character) (Variables|/Game/Variant_Shooter/Blueprints/BP_ShooterCharacter.BP_ShooterCharacter_C|GetMaxLvl _asbp_shooter_character))
    (Game|OpenLevel(byName) "BossLvl")
    (else
      (Game|OpenLevel(byName) "EasyLvl"))))

(fn ConstructionScript)