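; BP_DeathRay is a trap that moves a beam along a spline path and kills the player character on contact.
; A Timeline started on BeginPlay drives the Ray component's relative location along the Path spline and restarts from zero when finished, looping endlessly.
; Overlaps on the Collider that cast to BP_ShooterCharacter apply massive damage and print a warning message.
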(event OnComponentBeginOverlap(Collider)
  (params (OverlappedComponent :type Primitive%20Component%20Object%20Reference) (OtherActor :type Actor%20Object%20Reference) (OtherComp :type Primitive%20Component%20Object%20Reference) (OtherBodyIndex :type Integer) (bFromSweep :type Boolean) (SweepResult :type Hit%20Result%20Structure%20%28by%20ref%29))
  (bind _asbp_shooter_character (Utilities|Casting|CastToBP_ShooterCharacter OtherActor))
  (Game|Damage|ApplyDamage _asbp_shooter_character 9999.0 0 0 "/Script/Engine.DamageType")
  (Development|PrintText "Get away from the beam!"))

(event Custom|Move%20along
  (bind _новая_дорожка_0 (Timeline|Timeline Play)
    (:Update
      (Transformation|SetRelativeLocation (Variables|Default|GetRay) (Spline|GetLocationatTime (Variables|Default|GetPath) _новая_дорожка_0 "Local" false) false false))
    (:Finished
      (Components|Timeline|SetNewTime (Variables|Default|GetTimeline) 0.0)
      (Timeline|Timeline Play))))

(event EventBeginPlay
  (CallFunction|MoveAlong))

(fn ConstructionScript)